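; Game mode for MYTDS that runs a match countdown and ends the game when time runs out.
; BeginPlay starts a looping one-second timer that decrements GameTime.
; At zero it clears the timer, pauses the game, adds an end-game widget to the viewport and switches the Pc_MYTDS controller to UI-only input with the cursor visible.
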(event Custom|CustomEvent
  (bind _output_get (Variables|Default|SetGame%20Time (- (Variables|Default|GetGame%20Time) 1)))
  (if (== _output_get 0)
    (Utilities|Time|ClearandInvalidateTimerbyHandle (Variables|Default|GetTimer))
    (Game|SetGamePaused true)
    (bind _aspc_mytds (Utilities|Casting|CastToPc_MYTDS (Game|GetPlayerController 0)))
    (bind _returnvalue (UserInterface|CreateWidget "/Game/LeaveMeAlone/Widgets/UI/WBP_EndGame.WBP_EndGame_C"))
    (UserInterface|Viewport|AddtoViewport _returnvalue 0)
    (Input|SetInputModeUIOnly _aspc_mytds _returnvalue "DoNotLock" false)
    (Variables|/Script/Engine.PlayerController|SetbShowMouseCursor _aspc_mytds true)))

(event EventBeginPlay
  (bind _returnvalue (Utilities|Time|SetTimerbyEvent (delegate Custom|CustomEvent) 1.0 true))
  (Variables|Default|SetTimer _returnvalue))

(event EventTick
  (params (DeltaSeconds :type Float%20%28single-precision%29)))

(fn ConstructionScript)